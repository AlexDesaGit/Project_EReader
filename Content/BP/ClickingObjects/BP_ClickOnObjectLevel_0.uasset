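; BP_ClickOnObjectLevel_0 is a clickable object that briefly shows the WB_Level_0 widget when clicked.
; The click calls a custom event that creates the widget once, caches it in UserWidgetLevel0 and adds it to the viewport.
; A one-shot timer set to TimeToShowWidget then removes the widget from its parent.
; The construction script only calls the parent's version.
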(event `/Game/BP/Interfaces/IMouseClickOnObject.OnClick`
  ;[1 0 0.9171 1 40] On click
  (`self.OnClickCustomEvent`))

(event `OnClickCustomEvent`
  ;[1 1 1] Comment
  (`self.UserWidgetLevel_0`
    (:`then`
      _)
    (:`else`
      (bind _returnvalue (`|CreateWidget` "/Game/BP/Level_0/WB_Level_0.WB_Level_0_C"))
      (set `self.UserWidgetLevel_0` _returnvalue)))
  (`UserWidget.AddToViewport` (`self.UserWidgetLevel_0`) 0)
  (`KismetSystemLibrary.K2_SetTimerDelegate` (delegate `RemoveWidgetLevel_0FromParent`) (`self.TimeToShowWidget`)))

(event `RemoveWidgetLevel_0FromParent`
  ;[1 1 1] Comment
  (`Widget.RemoveFromParent` (`self.UserWidgetLevel_0`)))

(fn `UserConstructionScript`
  (`parent.UserConstructionScript`))